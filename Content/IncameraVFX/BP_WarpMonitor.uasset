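; BP_WarpMonitor is an in-camera VFX actor that supplies warp meshes for a four-screen display.
; On BeginPlay it assigns its Center, Left, Right and Upper mesh components to viewports vp_1 through vp_4 through the display API.
; Each assignment uses the actor's Root as the origin component, and the construction script is empty.
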(event `self.ReceiveBeginPlay`
  (`PicpProjectionBlueprintAPI.AssignWarpMeshToViewport` (`PicpProjectionIBlueprintLib.GetAPI`) "vp_1" (`self.center`) (`self.root`))
  (`PicpProjectionBlueprintAPI.AssignWarpMeshToViewport` (`PicpProjectionIBlueprintLib.GetAPI`) "vp_2" (`self.left`) (`self.root`))
  (`PicpProjectionBlueprintAPI.AssignWarpMeshToViewport` (`PicpProjectionIBlueprintLib.GetAPI`) "vp_3" (`self.right`) (`self.root`))
  (`PicpProjectionBlueprintAPI.AssignWarpMeshToViewport` (`PicpProjectionIBlueprintLib.GetAPI`) "vp_4" (`self.upper`) (`self.root`)))

(fn `UserConstructionScript`)