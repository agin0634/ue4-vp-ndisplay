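; In-camera VFX camera actor that drives a CineCamera from a VRPN tracker for an nDisplay inner-frustum viewport.
; Each Tick it assigns the camera to the viewport policy and applies the tracker pose, minus a calibration offset set by ResetOffset.
; It gets the viewport's render target from BP_IncameraStage and packs it into PICP blending parameters with soft edge.
; CaptureChromakey renders a scene capture matched to the camera's transform and FOV.
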(event `self.ReceiveBeginPlay`
  (bind _cameracomponent (`CameraActor.CameraComponent` (`self.CineCam`)))
  (`|ExecutionSequence`
    (:`then_0`
      (`|ExecutionSequence`
        (:`then_0`
          (`/Engine/EditorBlueprintResources/StandardMacros.IsValid` (`self.CineCam`)
            (:`Is Valid`
              (`SceneComponent.K2_SetRelativeLocationAndRotation` _cameracomponent (+ (`SceneComponent.RelativeLocation` _cameracomponent) (`self.TrackerLocationOffset`)) (`KismetMathLibrary.ComposeRotators` (`SceneComponent.RelativeRotation` _cameracomponent) (`self.TrackerRotationOffset`)) false false))
            (:`Is Not Valid`
              (`KismetSystemLibrary.PrintString` "Cine cam is not valid" true true (struct :`R` 1.0 :`G` 0.014578 :`A` 1.0)))))
        (:`then_1`
          (if (not (`self.bShowAxisDebug`))
            (`SceneComponent.SetVisibility` (`self.AxisMesh`) false false)))
        (:`then_2`
          (bind _returnvalue (`GameplayStatics.GetActorOfClass` "/Game/IncameraVFX/BP_nDisplayPawn.BP_nDisplayPawn_C"))
          (set `self.player` _returnvalue))))
    (:`then_1`
      (`|ExecutionSequence`
        (:`then_0`
          (bind _returnvalue_2 (`GameplayStatics.GetActorOfClass` "/Game/IncameraVFX/BP_IncameraStage.BP_IncameraStage_C"))
          (`/Engine/EditorBlueprintResources/StandardMacros.IsValid` _returnvalue_2
            (:`Is Valid`
              (set `self.IncameraStage` _returnvalue_2))
            (:`Is Not Valid`
              (`KismetSystemLibrary.PrintString` "StageSettings not found. Abort incamera rendering." true true (struct :`R` 1.0 :`B` 0.021864 :`A` 1.0) 5.0))))
        (:`then_1`
          (`self.Initialize Texture Render Targets`))))))

(event `ResetOffset`
  ;[1 1 1] TODO:check offset calculate
  (set `self.TrackerOffsetCalibration` (- (`SceneComponent.K2_GetComponentLocation` (`CameraActor.CameraComponent` (`self.CineCam`))) (`self.K2_GetActorLocation` (`self.player`)))))

(event `self.ReceiveTick`
  (params (DeltaSeconds :type "Float (single-precision)"))
  (bind _outapi (`DisplayClusterBlueprintLib.GetAPI`))
  (bind _vrpndeviceid (`self.VRPNDeviceID`))
  (bind _trackeroffsetcalibration (`self.TrackerOffsetCalibration`))
  (`|ExecutionSequence`
    (:`then_0`
      (`DisplayClusterProjectionBlueprintAPI.CameraPolicySetCamera` (`DisplayClusterProjectionBlueprintLib.GetAPI`) (`self.ViewportID`) (`CineCameraActor.GetCineCameraComponent` (`self.CineCam`)) 1.0))
    (:`then_1`
      (bind _location (`DisplayClusterBlueprintAPI.GetTrackerLocation` _outapi _vrpndeviceid 0))
      (`KismetSystemLibrary.PrintString` (`KismetStringLibrary.Conv_VectorToString` _trackeroffsetcalibration))
      (bind _rotation (`DisplayClusterBlueprintAPI.GetTrackerQuat` _outapi _vrpndeviceid 0))
      (bind _returnvalue (- _location _trackeroffsetcalibration))
      (bind _returnvalue_2 (`KismetMathLibrary.Quat_Rotator` _rotation))
      (`SceneComponent.K2_SetWorldLocationAndRotation` (`CameraActor.SceneComponent` (`self.CineCam`)) _returnvalue _returnvalue_2 false false)
      (`SceneComponent.K2_SetWorldLocationAndRotation` (`self.AxisMesh`) _returnvalue _returnvalue_2 false false))))

(fn `CaptureChromakey`
  (bind _cinecam (`self.CineCam`))
  (bind _scenecapturecomponent2d (`self.SceneCaptureComponent2D`))
  (set `SceneCaptureComponent2D.FOVAngle` (`CameraComponent.FieldOfView` (`CineCameraActor.GetCineCameraComponent` _cinecam)) _scenecapturecomponent2d)
  (`SceneComponent.K2_SetWorldLocationAndRotation` _scenecapturecomponent2d (`self.K2_GetActorLocation` _cinecam) (`self.K2_GetActorRotation` _cinecam) false false)
  (`SceneCaptureComponent2D.CaptureScene` (`self.SceneCaptureComponent2D`)))

(fn `GetBlendingParameters`
  (returns (Cameras :type "PicpCameraBlendingParameters Structure"))
  (`/Engine/EditorBlueprintResources/StandardMacros.IsValid` (`self.CineCam`)
    (:`Is Valid`
      (return (make `PicpCameraBlendingParameters` (`self.ReprojectedCineCam`) (`self.InnerCameraSoftEdge`) (`CineCameraActor.GetCineCameraComponent` (`self.CineCam`)) 1.0 (`self.ViewportID`))))
    (:`Is Not Valid`
      (return))))

(fn `Initialize Texture Render Targets`
  (`|ExecutionSequence`
    (:`then_0`
      (bind _newparam (`/Game/IncameraVFX/BP_IncameraStage.GetViewportRenderTarget` (`self.IncameraStage`) "rtt_inner_RT" (`self.ViewportID`) "RTF_RGB10A2"))
      (set `self.ReprojectedCineCam` _newparam))))

(fn `UserConstructionScript`)