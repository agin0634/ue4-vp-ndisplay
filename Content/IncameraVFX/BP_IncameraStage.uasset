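; In-camera VFX stage actor that configures nDisplay picp_mesh viewport overlays from projection data and BP_Incamera actors.
; At BeginPlay it registers as a projection listener, gathers those actors and creates cached per-viewport render targets.
; Projection updates store each frustum; the last viewport's update submits camera blending and Over-blended light card overlays.
; The custom-projection light card capture function exists but is never executed, and listener removal is unwired.
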(event `self.ReceiveBeginPlay`
  (`|ExecutionSequence`
    (:`then_0`
      (`PicpProjectionBlueprintAPI.AddProjectionDataListener` (`PicpProjectionIBlueprintLib.GetAPI`) self)
      (`self.InitializeRenderTargets`))
    (:`then_1`
      (bind _outactors (`GameplayStatics.GetAllActorsOfClass` "/Game/IncameraVFX/BP_Incamera.BP_Incamera_C"))
      (set `self.Incameras` _outactors))))

(event `self.ReceiveEndPlay`
  (params (EndPlayReason :type "EEndPlayReason Enum" :default "Destroyed"))
  (`self.ClearRenderTargetCache`))

(event `self.OnProjectionDataUpdate`
  (params (ProjectionData :type "PicpProjectionFrustumData Structure (by ref)"))
  (bind _lastprojectiondata (`self.Collect LightCards Frustums` ProjectionData))
  (if _lastprojectiondata
    (`self.SetupIncameraVFX`)))

(fn `CaptureLightCards`
  (bind _lightcardcapturecomponent (`self.LightCardCaptureComponent`))
  (for _array_element (`self.LCFRustumData`)
    (bind (_frustumdata _rendertexture) (break `/nDisplay/Blueprints/ReprojectionCamera/S_LightCardCaptureData` _array_element))
    (`SceneComponent.K2_SetWorldLocationAndRotation` _lightcardcapturecomponent (`.ViewLocation` (break `PicpProjectionFrustumData` _frustumdata)) (`.ViewRotation` (break `PicpProjectionFrustumData` _frustumdata)) false false)
    (set `SceneCaptureComponent2D.CustomProjectionMatrix` (`.PrjMatrix` (break `PicpProjectionFrustumData` _frustumdata)) _lightcardcapturecomponent)
    (set `SceneCaptureComponent2D.bUseCustomProjectionMatrix` true _lightcardcapturecomponent)
    (set `SceneCaptureComponent2D.TextureTarget` _rendertexture _lightcardcapturecomponent)
    (`SceneCaptureComponent2D.CaptureScene` (`self.LightCardCaptureComponent`)))
  (return))

(fn `Collect LightCards Frustums`
  (params (ProjectionData :type "PicpProjectionFrustumData Structure"))
  (returns (LastProjectionData :type Boolean))
  (bind _renderingviewportids (`self.RenderingViewportIDs`))
  (bind _projectiondata_id (break `PicpProjectionFrustumData` (`local.ProjectionData`)))
  (bind _returnvalue (`KismetArrayLibrary.Array_Find` (`self.RenderingViewportIDs`) (`.Id` (break `PicpProjectionFrustumData` ProjectionData))))
  (bind (_output_frustumdata _output_rendertexture) (break `/nDisplay/Blueprints/ReprojectionCamera/S_LightCardCaptureData` (`|GetArrayItem` (`self.LCFRustumData`) _returnvalue)))
  (`KismetArrayLibrary.Array_Set` (`self.LCFRustumData`) _returnvalue (make `/nDisplay/Blueprints/ReprojectionCamera/S_LightCardCaptureData` (`local.ProjectionData`) _output_rendertexture))
  (return (`KismetStringLibrary.EqualEqual_StrStr` (`|GetArrayItem` _renderingviewportids (`KismetArrayLibrary.Array_LastIndex` _renderingviewportids)) _projectiondata_id)))

(fn `GetOverlayBlendParameters`
  (returns (Overlays :type "Array of PicpOverlayFrameBlendingPair Structure"))
  (locals (LightCardOverlays :type "Array of PicpOverlayFrameBlendingPair Structure"))
  (for _array_element (`self.LCFRustumData`)
    (`KismetArrayLibrary.Array_Add` (`local.LightCardOverlays`) (make `PicpOverlayFrameBlendingPair` (break `PicpProjectionFrustumData` (break `/nDisplay/Blueprints/ReprojectionCamera/S_LightCardCaptureData` _array_element)) (`.RenderTexture_9_9E20C7D444F10668B8DE5CA383D45CF4` (break `/nDisplay/Blueprints/ReprojectionCamera/S_LightCardCaptureData` _array_element)))))
  (return (`local.LightCardOverlays`)))

(fn `GetViewportRenderTarget`
  (params (`Texture Name` :type String) (`Viewport Name` :type String) (Format :type "ETextureRenderTargetFormat Enum" :default "RTF_R8"))
  (returns (NewParam :type "TextureRenderTarget2D Object Reference"))
  (bind _returnvalue (`self.GetRenderTargetCached` `Texture Name`))
  (`/Engine/EditorBlueprintResources/StandardMacros.IsValid` _returnvalue
    (:`Is Valid`
      (return _returnvalue))
    (:`Is Not Valid`
      (bind (_viewportloc _viewportsize _returnvalue_2) (`DisplayClusterBlueprintAPI.GetViewportRect` (`DisplayClusterBlueprintLib.GetAPI`) (`local.Viewport Name`)))
      (if _returnvalue_2
        (bind _returnvalue_3 (`KismetRenderingLibrary.CreateRenderTarget2D` (break `IntPoint` _viewportsize) (`.Y` (break `IntPoint` _viewportsize)) (`local.Format`)))
        (`self.SetRenderTargetCached` (`local.Texture Name`) _returnvalue_3)
        (`KismetSystemLibrary.PrintString` (`KismetTextLibrary.Conv_TextToString` (`|FormatText` "PT {0} for {1}" (`KismetTextLibrary.Conv_StringToText` (`local.Texture Name`)) (`KismetTextLibrary.Conv_StringToText` (`local.Viewport Name`)))))
        (return _returnvalue_3)))))

(fn `InitializeRenderTargets`
  (bind (_viewportids _viewporttypes) (`DisplayClusterBlueprintAPI.GetLocalViewports` (`DisplayClusterBlueprintLib.GetAPI`) false))
  (for (_array_element _array_index) _viewportids
    (if (`KismetStringLibrary.EqualEqual_StrStr` (`|GetArrayItem` _viewporttypes _array_index) "picp_mesh")
      (bind _newparam (`self.GetViewportRenderTarget` (`KismetStringLibrary.Concat_StrStr` _array_element "_RT") _array_element "RTF_RG8"))
      (bind _s_lightcardcapturedata (make `/nDisplay/Blueprints/ReprojectionCamera/S_LightCardCaptureData` (make `PicpProjectionFrustumData` _array_element) _newparam))
      (`KismetArrayLibrary.Array_Add` (`self.LCFRustumData`) _s_lightcardcapturedata)
      (`KismetArrayLibrary.Array_Add` (`self.RenderingViewportIDs`) (break `PicpProjectionFrustumData` (`.FrustumData_12_2EED650B4184E2FF883BD1BF5F9B8A58` (break `/nDisplay/Blueprints/ReprojectionCamera/S_LightCardCaptureData` _s_lightcardcapturedata)))))))

(fn `SetupIncameraVFX`
  (locals (InCameraCapture :type "Array of PicpCameraBlendingParameters Structure"))
  (`|ExecutionSequence`
    (:`then_0`
      (for _array_element (`self.Incameras`)
        (`KismetArrayLibrary.Array_Add` (`local.InCameraCapture`) (`/Game/IncameraVFX/BP_Incamera.GetBlendingParameters` _array_element))))
    (:`then_1`
      (`PicpProjectionBlueprintAPI.SetupOverlayCaptures` (`PicpProjectionIBlueprintLib.GetAPI`) (`local.InCameraCapture`) (`self.GetOverlayBlendParameters`)))))

(fn `UserConstructionScript`)