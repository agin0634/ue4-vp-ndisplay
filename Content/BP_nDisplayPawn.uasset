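; BP_nDisplayPawn is a pawn, named for nDisplay setups, that forwards a keyboard reset to the in-camera rig.
; On BeginPlay it finds the BP_Incamera actor in the level and stores a reference.
; Pressing T calls ResetOffset on that actor.
; The remaining graph is empty stub events and an unconnected debug print of the root's world location.
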(event `self.ReceiveBeginPlay`
  (bind _returnvalue (`GameplayStatics.GetActorOfClass` "/Game/BP_Incamera.BP_Incamera_C"))
  (set `self.InCamera` _returnvalue))

(event `Key|T`
  (params (Key :type "Key Structure"))
  (:`Pressed`
    (`/Game/BP_Incamera.ResetOffset` (`self.InCamera`))))

(event `self.ReceiveTick`
  (params (DeltaSeconds :type "Float (single-precision)")))

(fn `UserConstructionScript`)