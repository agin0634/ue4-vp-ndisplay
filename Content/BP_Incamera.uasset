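; In-camera VFX actor that drives a cine camera from a VRPN tracker for an nDisplay viewport.
; Each tick it assigns the camera to the viewport policy and applies tracker position, minus a location offset, and rotation to the camera and debug axis mesh.
; ResetOffset recomputes that offset from camera and nDisplay pawn positions, marked TODO for checking.
; Stage lookup and render target initialization are unwired.
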(event `self.ReceiveBeginPlay`
  (`|ExecutionSequence`
    (:`then_0`
      (`|ExecutionSequence`
        (:`then_0`
          (`/Engine/EditorBlueprintResources/StandardMacros.IsValid` (`self.CineCam`)
            (:`Is Not Valid`
              (`KismetSystemLibrary.PrintString` "Cine cam is not valid" true true (struct :`R` 1.0 :`G` 0.014578 :`A` 1.0)))))
        (:`then_1`
          (if (not (`self.bShowAxisDebug`))
            (`SceneComponent.SetVisibility` (`self.AxisMesh`) false false)))
        (:`then_2`
          (bind _returnvalue (`GameplayStatics.GetActorOfClass` "/Game/BP_nDisplayPawn.BP_nDisplayPawn_C"))
          (set `self.player` _returnvalue))))))

(event `ResetOffset`
  ;[1 1 1] TODO:check offset calculate
  (set `self.LocationOffset` (- (`SceneComponent.K2_GetComponentLocation` (`CameraActor.CameraComponent` (`self.CineCam`))) (`self.K2_GetActorLocation` (`self.player`)))))

(event `self.ReceiveTick`
  (params (DeltaSeconds :type "Float (single-precision)"))
  (bind _outapi (`DisplayClusterBlueprintLib.GetAPI`))
  (bind _vrpndeviceid (`self.VRPNDeviceID`))
  (`|ExecutionSequence`
    (:`then_0`
      (`DisplayClusterProjectionBlueprintAPI.CameraPolicySetCamera` (`DisplayClusterProjectionBlueprintLib.GetAPI`) (`self.ViewportID`) (`CineCameraActor.GetCineCameraComponent` (`self.CineCam`)) 1.0))
    (:`then_1`
      ;[1 1 1] Comment
      (bind _location (`DisplayClusterBlueprintAPI.GetTrackerLocation` _outapi _vrpndeviceid 0))
      (bind _rotation (`DisplayClusterBlueprintAPI.GetTrackerQuat` _outapi _vrpndeviceid 0))
      (bind _returnvalue (- _location (`self.LocationOffset`)))
      (bind _returnvalue_2 (`KismetMathLibrary.Quat_Rotator` _rotation))
      (`SceneComponent.K2_SetRelativeLocationAndRotation` (`Actor.RootComponent` (`self.CineCam`)) _returnvalue _returnvalue_2 false false)
      (`SceneComponent.K2_SetRelativeLocationAndRotation` (`self.AxisMesh`) _returnvalue _returnvalue_2 false false))))

(fn `Initialize Texture Render Targets`
  (`/Game/BP_IncameraStage.GetViewportRenderTarget` (`self.IncameraStage`) "rtt_inner_RT" "rtt_inner"))

(fn `UserConstructionScript`)