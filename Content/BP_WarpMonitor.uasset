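; BP_WarpMonitor is an actor that registers warp meshes for a three-viewport display setup, apparently nDisplay.
; On BeginPlay it calls the API's AssignWarpMeshToViewport to bind its Center, Left and Right mesh components to viewports vp_1, vp_2 and vp_3.
; All three assignments use the actor's Root component as the warp origin.
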(event `self.ReceiveBeginPlay`
  (`PicpProjectionBlueprintAPI.AssignWarpMeshToViewport` (`PicpProjectionIBlueprintLib.GetAPI`) "vp_1" (`self.center`) (`self.root`))
  (`PicpProjectionBlueprintAPI.AssignWarpMeshToViewport` (`PicpProjectionIBlueprintLib.GetAPI`) "vp_2" (`self.left`) (`self.root`))
  (`PicpProjectionBlueprintAPI.AssignWarpMeshToViewport` (`PicpProjectionIBlueprintLib.GetAPI`) "vp_3" (`self.right`) (`self.root`)))

(fn `UserConstructionScript`)