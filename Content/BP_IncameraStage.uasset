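; In-camera stage actor for nDisplay that registers as a projection data listener on BeginPlay, then clears its render target cache and unregisters on EndPlay.
; InitializeRenderTargets finds local "picp_mesh" viewports and requests a render target for each.
; GetViewportRenderTarget returns the cached target, or creates, caches and logs one sized to the viewport rect.
; InitializeRenderTargets is only called from an unconnected node in the event graph, so it never runs there.
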(event `self.ReceiveBeginPlay`
  (`PicpProjectionBlueprintAPI.AddProjectionDataListener` (`PicpProjectionIBlueprintLib.GetAPI`) self))

(event `self.ReceiveEndPlay`
  (params (EndPlayReason :type "EEndPlayReason Enum" :default "Destroyed"))
  (`self.ClearRenderTargetCache`)
  (`PicpProjectionBlueprintAPI.RemoveProjectionDataListener` (`PicpProjectionIBlueprintLib.GetAPI`) self))

(fn `GetViewportRenderTarget`
  (params (`Texture Name` :type String) (`Viewport Name` :type String))
  (returns (NewParam :type "TextureRenderTarget2D Object Reference"))
  (bind _returnvalue (`self.GetRenderTargetCached` `Texture Name`))
  (`/Engine/EditorBlueprintResources/StandardMacros.IsValid` _returnvalue
    (:`Is Valid`
      (return _returnvalue))
    (:`Is Not Valid`
      (bind (_viewportloc _viewportsize _returnvalue_2) (`DisplayClusterBlueprintAPI.GetViewportRect` (`DisplayClusterBlueprintLib.GetAPI`) (`local.Viewport Name`)))
      (if _returnvalue_2
        (bind _returnvalue_3 (`KismetRenderingLibrary.CreateRenderTarget2D` (break `IntPoint` _viewportsize) (`.Y` (break `IntPoint` _viewportsize)) "RTF_RGBA8"))
        (`self.SetRenderTargetCached` (`local.Texture Name`) _returnvalue_3)
        (`KismetSystemLibrary.PrintString` (`KismetTextLibrary.Conv_TextToString` (`|FormatText` "PT {0} for {1}" (`KismetTextLibrary.Conv_StringToText` (`local.Texture Name`)) (`KismetTextLibrary.Conv_StringToText` (`local.Viewport Name`)))))
        (return _returnvalue_3)))))

(fn `InitializeRenderTargets`
  (bind (_viewportids _viewporttypes) (`DisplayClusterBlueprintAPI.GetLocalViewports` (`DisplayClusterBlueprintLib.GetAPI`) false))
  (for (_array_element _array_index) _viewportids
    (if (`KismetStringLibrary.EqualEqual_StrStr` (`|GetArrayItem` _viewporttypes _array_index) "picp_mesh")
      (`self.GetViewportRenderTarget` (`KismetStringLibrary.Concat_StrStr` _array_element "_RT") _array_element))))

(fn `UserConstructionScript`)